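; Player-controlled tank Blueprint that binds input to camera aiming, firing and differential left/right drive.
; On BeginPlay it hands its barrel, turret and gear head components to reference setters defined outside these graphs.
; Aim axes rotate an azimuth gimbal for yaw and a spring arm for pitch, rather than turning the turret directly.
; Separate thruster axes set throttle on the left and right rear leg components, and the Fire action calls Fire.
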(event EventBeginPlay
  (Class|Tank|SetBarrelReference (Variables|Default|GetBarrel))
  (Class|Tank|SetTurretReference (Variables|Default|GetTankTurret))
  (Class|Tank|SetGearHeadReference (Variables|Default|GetGearHead)))

(event Input|ActionEvents|InputActionFire
  (params (Key :type Key%20Structure))
  (:Pressed
    (Class|Tank|Fire)))

(event Input|AxisEvents|InputAxisAimAzimuth
  (params (AxisValue :type Float%20%28single-precision%29))
  (Transformation|AddLocalRotation (Variables|Default|GetAzimuth%20Gimbal) (Math|Rotator|MakeRotator 0.0 0.0 AxisValue) false false))

(event Input|AxisEvents|InputAxisAimElevation
  (params (AxisValue :type Float%20%28single-precision%29))
  (Transformation|AddLocalRotation (Variables|Default|GetPitchSpringArm) (Math|Rotator|MakeRotator 0.0 AxisValue 0.0) false false))

(event Input|AxisEvents|InputAxisLeftThruster
  (params (AxisValue :type Float%20%28single-precision%29))
  (Class|TankRearLeg|SetThrottle (Variables|Default|GetTankRearLeg_LH) AxisValue))

(event Input|AxisEvents|InputAxisRightThruster
  (params (AxisValue :type Float%20%28single-precision%29))
  (Class|TankRearLeg|SetThrottle (Variables|Default|GetTankRearLeg_RH) AxisValue))

(fn ConstructionScript)